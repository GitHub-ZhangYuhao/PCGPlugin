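; BP_Building is a procedural building actor that configures its PCG graph instance from wall size, floor size, wall thickness and floor count.
; The Construction Script derives floor offset and scale, four axis-aligned wall offsets, a wall pivot offset and building height, then writes them as graph parameters.
; It also flags single-floor buildings for the graph, and the actor has no active runtime logic.
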(event EventBeginPlay)

(event Collision|EventActorBeginOverlap
  (params (OtherActor :type Actor%20Object%20Reference)))

(event EventTick
  (params (DeltaSeconds :type Float%20%28single-precision%29)))

(fn ConstructionScript
  (bind _floorsize (Variables|Default|GetFloorSize))
  (bind _returnvalue (/ _floorsize -2.0))
  (Utilities|FlowControl|Sequence
    (:then_0
      (Variables|Default|SetPCGInstance (Variables|/Script/PCG.PCGComponent|GetGraphInstance (Variables|Default|GetPCG))))
    (:then_1
      (Effects|Components|ParticleSystem|SetFloatParameter (Variables|Default|GetPCGInstance) "WallSize" (Variables|Default|GetWallSize))
      ;[1 1 1] FloorOffset
      (bind _output_get (Variables|Default|SetFloorOffset (Math|Vector|MakeVector _returnvalue _returnvalue 0.0)))
      (Effects|Components|ParticleSystem|SetVectorParameter (Variables|Default|GetPCGInstance) "FloorOffset" _output_get)
      ;[1 1 1] FloorScale
      (bind _output_get_2 (Variables|Default|SetFloorScale (/ (Variables|Default|GetWallSize) (Variables|Default|GetFloorSize))))
      (Effects|Components|ParticleSystem|SetVectorParameter (Variables|Default|GetPCGInstance) "FloorScale" (Math|Conversions|ToVector(Float) _output_get_2))
      ;[0.15 0.15 0.15] WallOffset PCGParam
      (Variables|Default|SetWallOffsetDistance (/ (* (Variables|Default|GetFloorScale) (Variables|Default|GetFloorSize)) 2.0))
      (Effects|Components|ParticleSystem|SetVectorParameter (Variables|Default|GetPCGInstance) "WallOffset01" (Math|Vector|MakeVector (* (Variables|Default|GetWallOffsetDistance) -1.0) 0.0 0.0))
      (Effects|Components|ParticleSystem|SetVectorParameter (Variables|Default|GetPCGInstance) "WallOffset02" (Math|Vector|MakeVector (Variables|Default|GetWallOffsetDistance) 0.0 0.0))
      (Effects|Components|ParticleSystem|SetVectorParameter (Variables|Default|GetPCGInstance) "WallOffset03" (Math|Vector|MakeVector 0.0 (* (Variables|Default|GetWallOffsetDistance) -1.0) 0.0))
      (Effects|Components|ParticleSystem|SetVectorParameter (Variables|Default|GetPCGInstance) "WallOffset04" (Math|Vector|MakeVector 0.0 (Variables|Default|GetWallOffsetDistance) 0.0))
      (Effects|Components|ParticleSystem|SetVectorParameter (Variables|Default|GetPCGInstance) "WallOffsetPivot" (Math|Vector|MakeVector (/ (Variables|Default|GetWallSize) -2.0) (Variables|Default|GetWallTickness) 0.0))
      (Effects|Components|ParticleSystem|SetVectorParameter (Variables|Default|GetPCGInstance) "BuildingHeight" (Math|Vector|MakeVector 0.0 0.0 (* (Variables|Default|GetWallSize) (- (Variables|Default|GetFloors) 1))))
      (Effects|Components|ParticleSystem|SetBoolParameter (Variables|Default|GetPCGInstance) "bSingleFloor" (<= (Variables|Default|GetFloors) 1)))))