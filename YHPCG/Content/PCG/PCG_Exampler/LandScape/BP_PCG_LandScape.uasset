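; Custom PCG Blueprint node that sets point density from landscape paint layer weights.
; ExecuteWithContext converts the first spatial input to points, stores its target actor as world context, and runs the point loop.
; Each point samples interpolated layer weights at its location, taking the weight as density if the name matches LayerName, otherwise zero.
; Both branches return inside the loop, so only the first returned layer is ever compared.
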(fn ExecutewithContext
  (params (InContext :type PCG%20Context%20Structure%20%28by%20ref%29) (Input :type PCG%20Data%20Collection%20Structure%20%28by%20ref%29))
  (bind _returnvalue (Class|PCGDataFunctionLibrary|GetInputs Input))
  (bind _aspcgspatial_data (Utilities|Casting|CastToPCGSpatialData (.Data (Utilities|Struct|BreakPCGTaggedData (Utilities|Array|Get(acopy) _returnvalue))))
    (:then
      (bind _returnvalue_2 (Class|PCGBlueprintHelpers|GetTargetActor InContext _aspcgspatial_data))
      (Variables|Default|SetTarget%20Actor _returnvalue_2)
      (bind _outdata (PCG|FlowControl|PointLoop InContext (SpatialData|ToPointDatawithContext _aspcgspatial_data InContext) 0)))
    (:CastFailed
      _))
  (return (Utilities|Struct|MakePCGDataCollection (Utilities|Array|MakeArray (Utilities|Struct|MakePCGTaggedData _outdata 0 "None")))))

(fn PointLoopBody
  (params (InContext :type PCG%20Context%20Structure%20%28by%20ref%29) (InData :type PCG%20Point%20Data%20Object%20Reference) (InPoint :type PCG%20Point%20Structure%20%28by%20ref%29) (OutMetadata :type PCG%20Metadata%20Object%20Reference))
  (bind _returnvalue (Class|PCGBlueprintHelpers|GetInterpolatedPCGLandscapeLayerWeights (Variables|Default|GetTarget%20Actor) (.Location (Math|Transform|BreakTransform (.Transform (Utilities|Struct|BreakPCGPoint InPoint))))))
  (for _array_element _returnvalue
    (if (== (.Name (Utilities|Struct|BreakPCGLandscapeLayerWeight _array_element)) (Variables|Default|GetLayerName))
      (bind _structout (Utilities|Struct|SetmembersinPCGPoint InPoint (.Weight (Utilities|Struct|BreakPCGLandscapeLayerWeight _array_element))))
      (return _structout true)
      (else
        (bind _structout_2 (Utilities|Struct|SetmembersinPCGPoint InPoint 0.0))
        (return _structout_2 true)))))