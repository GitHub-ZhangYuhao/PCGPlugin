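; BP_PCG_CustomNode is an example custom PCG Blueprint node that turns point density into box height and randomizes point color.
; It converts the first input's spatial data to points and runs a point loop over them.
; Each point keeps its minimum bounds, gets a fixed XY maximum with Z set to density times MaxHeight, and takes color from random unit vectors.
; The modified points are returned as a new data collection.
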(fn ExecutewithContext
  (params (InContext :type PCG%20Context%20Structure%20%28by%20ref%29) (Input :type PCG%20Data%20Collection%20Structure%20%28by%20ref%29))
  (bind _returnvalue (Class|PCGDataFunctionLibrary|GetInputs Input))
  (bind _aspcgspatial_data (Utilities|Casting|CastToPCGSpatialData (.Data (Utilities|Struct|BreakPCGTaggedData (Utilities|Array|Get(acopy) _returnvalue))))
    (:then
      (bind _outdata (PCG|FlowControl|PointLoop InContext (SpatialData|ToPointDatawithContext _aspcgspatial_data InContext) 0)))
    (:CastFailed
      _))
  (return (Utilities|Struct|MakePCGDataCollection (Utilities|Array|MakeArray (Utilities|Struct|MakePCGTaggedData _outdata 0 "None")))))

(fn PointLoopBody
  (params (InContext :type PCG%20Context%20Structure%20%28by%20ref%29) (InData :type PCG%20Point%20Data%20Object%20Reference) (InPoint :type PCG%20Point%20Structure%20%28by%20ref%29) (OutMetadata :type PCG%20Metadata%20Object%20Reference))
  (bind (_transform _density _boundsmin) (Utilities|Struct|BreakPCGPoint InPoint))
  (bind _returnvalue (Math|Random|RandomUnitVector))
  (bind _structout (Utilities|Struct|SetmembersinPCGPoint InPoint _boundsmin (Math|Vector|MakeVector 5e+01 5e+01 (* _density (Variables|Default|GetMaxHeight))) (Math|Vector4|MakeVector4 (.x _returnvalue) (.y _returnvalue) (.z _returnvalue) 1.0)))
  (return _structout true))